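; Player controller Blueprint for an action roguelike that sets up the local player's HUD and offers a save hotkey.
; When the playing state begins on a local controller, it creates the Main_HUD widget, adds it to the viewport and switches input to game-only.
; Pressing L casts the game mode to SGameModeBase, writes the save game and prints a confirmation message.
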(event EventBlueprintBeginPlayingState
  (if (Pawn|IsLocalController)
    (bind _returnvalue (UserInterface|CreateWidget "/Game/ActionRougelike/UI/Main_HUD.Main_HUD_C"))
    (UserInterface|Viewport|AddtoViewport _returnvalue 0)
    (Input|SetInputModeGameOnly self)))

(event EventBeginPlay)

(event Input|KeyboardEvents|L
  (params (Key :type Key%20Structure :default "None"))
  (:Pressed
    (bind _assgame_mode_base (Utilities|Casting|CastToSGameModeBase (Game|GetGameMode)))
    (Class|SGameModeBase|WriteSaveGame _assgame_mode_base)
    (Development|PrintString "Save World!")))

(fn ConstructionScript)